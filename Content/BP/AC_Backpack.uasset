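; Backpack inventory component that stores items as an array of ID/count stacks, with max stack size and type looked up by ID.
; Adding tops up the first non-full matching stack, then spills the remainder into new stacks.
; Dropping removes part or all of a stack (-1 means all); both operations fire dispatchers.
; Queries return items tagged with their array index, optionally filtered by type.
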(event EventBeginPlay)

(event EventTick
  (params (DeltaSeconds :type Float%20%28single-precision%29)))

(fn GetItemsCF
  (for (_array_element _array_index) (Variables|Default|GetItems)
    (Utilities|Array|Add (LocalVariables|GetNewLocalVar_0) (Utilities|Struct|MakeStruct_BackpackItemsIndex (.ID (Utilities|Struct|BreakStruct_BackpackItems _array_element)) (.Number (Utilities|Struct|BreakStruct_BackpackItems _array_element)) _array_index)))
  (return (LocalVariables|GetNewLocalVar_0)))

(fn AddItemsCF
  (params (ID :type Name) (Number :type Integer))
  (bind _输出行 (CallFunction|GetTargetItemFCL ID))
  (bind _最大数量 (Utilities|Struct|BreakStruct_Items _输出行))
  (LocalVariables|SetLocalNumber Number)
  (bind (_index _return) (CallFunction|FindItemCF ID true))
  (if _return
    (bind _output_get (LocalVariables|SetLocalIndexArray _index))
    (bind _array_element (Utilities|Array|ForEachLoopwithBreak _output_get :!label _label)
      (:LoopBody
        (LocalVariables|SetLocalIndex _array_element)
        (if (>= (.Number (Utilities|Struct|BreakStruct_BackpackItems (Utilities|Array|Get(acopy) (Variables|Default|GetItems) (LocalVariables|GetLocalIndex)))) _最大数量)
          (goto _label Break)
          (elif (>= (- _最大数量 (+ (.Number (Utilities|Struct|BreakStruct_BackpackItems (Utilities|Array|Get(acopy) (Variables|Default|GetItems) (LocalVariables|GetLocalIndex)))) (LocalVariables|GetLocalNumber))) 0)
            (Utilities|Array|SetArrayElem (Variables|Default|GetItems) (LocalVariables|GetLocalIndex) (Utilities|Struct|MakeStruct_BackpackItems ID (+ (.Number (Utilities|Struct|BreakStruct_BackpackItems (Utilities|Array|Get(acopy) (Variables|Default|GetItems) (LocalVariables|GetLocalIndex)))) (LocalVariables|GetLocalNumber))) true)
            (Default|CallAddDisCS)
            (return)
            (else
              (LocalVariables|SetLocalNumber (Math|Integer|Absolute(Integer) (- _最大数量 (+ (.Number (Utilities|Struct|BreakStruct_BackpackItems (Utilities|Array|Get(acopy) (Variables|Default|GetItems) (LocalVariables|GetLocalIndex)))) (LocalVariables|GetLocalNumber)))))
              (Utilities|Array|SetArrayElem (Variables|Default|GetItems) (LocalVariables|GetLocalIndex) (Utilities|Struct|MakeStruct_BackpackItems ID (Utilities|Struct|BreakStruct_Items (CallFunction|GetTargetItemFCL ID))) true)
              (goto _label Break)))))
      (:Completed
        _)))
  (while (> (- (LocalVariables|GetLocalNumber) (Utilities|Struct|BreakStruct_Items (CallFunction|GetTargetItemFCL ID))) 0)
    (Utilities|Array|Add (Variables|Default|GetItems) (Utilities|Struct|MakeStruct_BackpackItems ID (Utilities|Struct|BreakStruct_Items (CallFunction|GetTargetItemFCL ID))))
    (LocalVariables|SetLocalNumber (- (LocalVariables|GetLocalNumber) (Utilities|Struct|BreakStruct_Items (CallFunction|GetTargetItemFCL ID)))))
  (Utilities|Array|Add (Variables|Default|GetItems) (Utilities|Struct|MakeStruct_BackpackItems ID (LocalVariables|GetLocalNumber)))
  (Default|CallAddDisCS)
  (return))

(fn FindItemCF
  (params (ID :type Name) (最大数量 :type Boolean))
  (bind _localindexarray (LocalVariables|GetLocalIndexArray))
  (for (_array_element _array_index) (Variables|Default|GetItems)
    (if (Utilities|Name|Equal(Name) (.ID (Utilities|Struct|BreakStruct_BackpackItems _array_element)) ID)
      (if 最大数量
        (if (not (>= (.Number (Utilities|Struct|BreakStruct_BackpackItems _array_element)) (Utilities|Struct|BreakStruct_Items (CallFunction|GetTargetItemFCL ID))))
          (Utilities|Array|Add (LocalVariables|GetLocalIndexArray) _array_index :!label _label))
        (else
          (goto _label)))))
  (return _localindexarray (Utilities|Array|IsValidIndex _localindexarray)))

(fn DropItemCF
  (params (ItemIndex :type Integer) (Number :type Integer))
  (bind _items (Variables|Default|GetItems))
  (bind _output (Utilities|Array|Get(acopy) _items ItemIndex))
  (bind (_id _number) (Utilities|Struct|BreakStruct_BackpackItems _output))
  (if (or (== Number -1) (<= (.Number (Utilities|Struct|BreakStruct_BackpackItems (Utilities|Array|Get(acopy) (Variables|Default|GetItems) ItemIndex))) Number))
    (Default|CallDropDisCS (Utilities|Array|Get(acopy) (Variables|Default|GetItems) ItemIndex))
    (Utilities|Array|RemoveIndex (Variables|Default|GetItems) ItemIndex)
    (else
      (Default|CallDropDisCS (Utilities|Struct|MakeStruct_BackpackItems _id Number))
      (Utilities|Array|SetArrayElem (Variables|Default|GetItems) ItemIndex (Utilities|Struct|MakeStruct_BackpackItems _id (- _number Number)) true))))

(fn GetTargetTypeItemsCF
  (params (ItemType :type Enum_ItemsType%20Enum :default "NewEnumerator0"))
  (if (Utilities|Enum|Equal(Enum) ItemType "NewEnumerator0")
    (return (CallFunction|GetItemsCF))
    (else
      (for (_array_element _array_index) (Variables|Default|GetItems)
        (if (== ItemType (Utilities|Struct|BreakStruct_Items (CallFunction|GetTargetItemFCL (.ID (Utilities|Struct|BreakStruct_BackpackItems _array_element)))))
          (Utilities|Array|Add (LocalVariables|GetNewLocalVar_0) (Utilities|Struct|MakeStruct_BackpackItemsIndex (.ID (Utilities|Struct|BreakStruct_BackpackItems _array_element)) (.Number (Utilities|Struct|BreakStruct_BackpackItems _array_element)) _array_index))))
      (return (LocalVariables|GetNewLocalVar_0)))))
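; Player character that carries an inventory through a backpack component, with B toggling a lazily created backpack widget and the mouse cursor.
; Wrapper functions forward add, drop, item query and capacity calls to the component, and the component's drop event spawns a BP_Item in front of the character.
; Adding from an item actor destroys it if everything fits, otherwise writes back the returned count.
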(event Collision|EventActorBeginOverlap
  (params (OtherActor :type Actor%20Object%20Reference)))

(event EventTick
  (params (DeltaSeconds :type Float%20%28single-precision%29)))

(event DropDisCS(AC_Backpack)
  (params (BackpackItem :type Struct%20Backpack%20Items%20Structure))
  (bind _mesh (Variables|Character|GetMesh))
  (bind _returnvalue (Transformation|GetWorldTransform _mesh))
  (bind (_location _rotation _scale) (Math|Transform|BreakTransform _returnvalue))
  (Game|SpawnActorfromClass "/Game/Items/BP/BP_Item.BP_Item_C" (Math|Transform|MakeTransform (+ _location (* (Transformation|GetActorForwardVector) 88.0)) _rotation _scale) "AdjustIfPossibleButDontSpawnIfColliding" 0 BackpackItem 0))

(event Custom|Spawn
  (Game|SpawnActorfromClass :Class "/Game/Items/BP/BP_Item_Blue.BP_Item_Blue_C" :SpawnTransform (Math|Transform|MakeTransform "0, 0, 0") :CollisionHandlingOverride "AlwaysSpawn" :Instigator 0))

(event EventBeginPlay
  (Variables|/Script/Engine.PlayerController|SetbShowMouseCursor (Game|GetPlayerController 0) true))

(event Input|KeyboardEvents|B
  (params (Key :type Key%20Structure))
  (bind _returnvalue (Game|GetPlayerController 0))
  (:Pressed
    (Utilities|IsValid (Variables|Default|GetWB_Backpack)
      (:Is%20Valid
        (if (UserInterface|Viewport|IsinViewport (Variables|Default|GetWB_Backpack))
          (Widget|RemovefromParent (Variables|Default|GetWB_Backpack))
          (Variables|/Script/Engine.PlayerController|SetbShowMouseCursor _returnvalue false)
          (else
            (UserInterface|Viewport|AddtoViewport (Variables|Default|GetWB_Backpack) 0 :!label _label)
            (Variables|/Script/Engine.PlayerController|SetbShowMouseCursor _returnvalue true))))
      (:Is%20Not%20Valid
        (bind _returnvalue_2 (UserInterface|CreateWidget "/Game/Widget/WB_Backpack.WB_Backpack_C"))
        (Variables|Default|SetWB_Backpack _returnvalue_2)
        (goto _label)))))

(fn ConstructionScript)

(fn GetBackpackItemsCF
  (return (Default|GetItemsCF (Variables|Default|GetAC_Backpack))))

(fn AddItemsCF
  (params (ID :type Name) (Number :type Integer))
  (bind (_alladd _ruturnnum) (Default|AddItemsCF (Variables|Default|GetAC_Backpack) ID Number))
  (return _alladd _ruturnnum))

(fn AddItemsActorCF
  (params (Item :type BP%20Item%20Object%20Reference%20%28by%20ref%29))
  (bind _backpackitem (Variables|/Game/Items/BP/BP_Item.BP_Item_C|GetBackpackItem Item))
  (bind (_id _number) (Utilities|Struct|BreakStruct_BackpackItems _backpackitem))
  (bind (_alladd _ruturnnum) (Default|AddItemsCF (Variables|Default|GetAC_Backpack) _id _number))
  (if _alladd
    (Actor|DestroyActor Item)
    (else
      (Default|SetNewNumCF Item _ruturnnum)))
  (return))

(fn DropItemCF
  (params (ItemIndex :type Integer) (Number :type Integer))
  (Default|DropItemCF (Variables|Default|GetAC_Backpack) ItemIndex Number))

(fn GetTargetTypeItemsCF
  (params (ItemType :type Enum_ItemsType%20Enum :default "NewEnumerator0"))
  (return (Default|GetTargetTypeItemsCF (Variables|Default|GetAC_Backpack) ItemType)))

(fn GetCapacityCF
  (bind _ac_backpack (Variables|Default|GetAC_Backpack))
  (return (Variables|/Game/BP/AC_Backpack.AC_Backpack_C|GetAllSize _ac_backpack) (Variables|/Game/BP/AC_Backpack.AC_Backpack_C|GetCapacity _ac_backpack)))
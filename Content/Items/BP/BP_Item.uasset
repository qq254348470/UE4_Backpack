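; BP_Item is an item actor that represents a backpack item, holding an ID and a count in a BackpackItem struct.
; Its construction script adds a static mesh component and sets its mesh from the item data looked up by ID.
; Two functions rebuild the struct to either subtract from or overwrite the count, and the event graph has no active logic.
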(event EventBeginPlay)

(event Collision|EventActorBeginOverlap
  (params (OtherActor :type Actor%20Object%20Reference)))

(event EventTick
  (params (DeltaSeconds :type Float%20%28single-precision%29)))

(fn ConstructionScript
  (bind _returnvalue (AddComponent|AddStaticMeshComponent false))
  (Components|StaticMesh|SetStaticMesh _returnvalue (.模型 (Utilities|Struct|BreakStruct_Items (CallFunction|GetTargetItemFCL (.ID (Utilities|Struct|BreakStruct_BackpackItems (Variables|Default|GetBackpackItem))))))))

(fn RemoveNumCF
  (params (Number :type Integer))
  (Variables|Default|SetBackpackItem (Utilities|Struct|MakeStruct_BackpackItems (.ID (Utilities|Struct|BreakStruct_BackpackItems (Variables|Default|GetBackpackItem))) (- (.Number (Utilities|Struct|BreakStruct_BackpackItems (Variables|Default|GetBackpackItem))) Number))))

(fn SetNewNumCF
  (params (Number :type Integer))
  (Variables|Default|SetBackpackItem (Utilities|Struct|MakeStruct_BackpackItems (.ID (Utilities|Struct|BreakStruct_BackpackItems (Variables|Default|GetBackpackItem))) Number)))
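; BP_Character is a player pawn Blueprint that provides a keyboard-toggled backpack UI.
; Its Backpack graph shows player 0's mouse cursor on BeginPlay.
; Pressing B creates a WB_Temp widget on first use, caches it as WBBackpack, then toggles it on and off the viewport.
; The main EventGraph holds only disabled placeholder events, and the construction script is empty.
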(event EventBeginPlay)

(event Collision|EventActorBeginOverlap
  (params (OtherActor :type Actor%20Object%20Reference)))

(event EventTick
  (params (DeltaSeconds :type Float%20%28single-precision%29)))

(event EventBeginPlay
  (Variables|/Script/Engine.PlayerController|SetbShowMouseCursor (Game|GetPlayerController 0) true))

(event Input|KeyboardEvents|B
  (params (Key :type Key%20Structure))
  (:Pressed
    (Utilities|IsValid (Variables|Default|GetWB_Backpack)
      (:Is%20Valid
        (if (UserInterface|Viewport|IsinViewport (Variables|Default|GetWB_Backpack))
          (Widget|RemovefromParent (Variables|Default|GetWB_Backpack))
          (else
            (UserInterface|Viewport|AddtoViewport (stale _output_get) 0 :!label _label))))
      (:Is%20Not%20Valid
        (bind _returnvalue (UserInterface|CreateWidget "/Game/Widget/WB_Temp.WB_Temp_C"))
        (bind _output_get (Variables|Default|SetWB_Backpack _returnvalue))
        (goto _label)))))

(fn ConstructionScript)
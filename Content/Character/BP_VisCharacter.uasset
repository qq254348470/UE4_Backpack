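; BP_VisCharacter is a visualization actor with a scene capture that shows only its own components, plus mouse-driven picking.
; Construction sets the show-only list and derives Distance from the camera's absolute relative Y.
; InputMousePosition_CS scales incoming coordinates to move a Cube and offset a debug-drawn complex Visibility trace along camera forward, reaching slightly beyond Distance.
; The trace can hit the actor itself, but its result triggers nothing yet.
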(event Custom|InputMousePosition_CS
  (params (X :type Float%20%28single-precision%29) (Y :type Float%20%28single-precision%29))
  (bind _returnvalue (* Y 0.63))
  (bind _returnvalue_2 (* X 0.63))
  (bind _camera (Variables|Default|GetCamera))
  (bind _returnvalue_3 (Transformation|GetWorldLocation _camera))
  (bind _returnvalue_4 (+ (Math|Vector|MakeVector 0.0 _returnvalue_2 _returnvalue) _returnvalue_3))
  (Transformation|SetRelativeLocation (Variables|Default|GetCube) (Math|Vector|MakeVector 0.0 _returnvalue_2 _returnvalue) false false)
  (bind (_outhit _returnvalue_5) (Collision|LineTraceByChannel _returnvalue_4 (+ _returnvalue_4 (* (Math|Vector|GetForwardVector _camera) (+ (Variables|Default|GetDistance) 5e+01))) "TraceTypeQuery1" true 0 "ForDuration" false))
  (if _returnvalue_5
    _))

(event EventBeginPlay)

(event Collision|EventActorBeginOverlap
  (params (OtherActor :type Actor%20Object%20Reference)))

(event EventTick
  (params (DeltaSeconds :type Float%20%28single-precision%29)))

(fn ConstructionScript
  (Rendering|SceneCapture|ShowOnlyActorComponents (Variables|Default|GetSceneCaptureComponent2D) self)
  (Variables|Default|SetDistance (Math|Float|Absolute(Float) (.y (Variables|/Script/Engine.SceneComponent|GetRelativeLocation (Variables|Default|GetCamera))))))